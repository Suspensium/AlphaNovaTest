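; BP_GameState tracks painting progress across the level's targets and detects the win condition.
; CountTargets resets the counters, then tallies BP_Purifier and BP_DefaultTarget actors by their Painted flag using GetAllActorsOfClass scans.
; HasWon runs after each tally; when no unpainted purifiers or default targets remain, it shows WBP_Win, removes WBP_TargetsInfo and disables input on the player's pawn.
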(event `Count Targets`
  (set `self.PurifiersCount` 0)
  (set `self.PaintedCount` 0)
  (set `self.UnpaintedCount` 0)
  (`self.Count Purifiers`)
  (`self.Count Default Targets`)
  (`self.Has Won`))

(event `Count Purifiers`
  (bind _outactors (`GameplayStatics.GetAllActorsOfClass` "/Game/AlphaNovaTest/Core/Actors/BP_Purifier.BP_Purifier_C"))
  (for _array_element _outactors
    (if (not (`CPP_Target.bPainted` _array_element))
      (`/Engine/EditorBlueprintResources/StandardMacros.IncrementInt` (`self.PurifiersCount`))
      (else
        (`/Engine/EditorBlueprintResources/StandardMacros.IncrementInt` (`self.PaintedCount`))))))

(event `Count Default Targets`
  (bind _outactors (`GameplayStatics.GetAllActorsOfClass` "/Game/AlphaNovaTest/Core/Actors/BP_DefaultTarget.BP_DefaultTarget_C"))
  (for _array_element _outactors
    (if (not (`CPP_Target.bPainted` _array_element))
      (`/Engine/EditorBlueprintResources/StandardMacros.IncrementInt` (`self.UnpaintedCount`))
      (else
        (`/Engine/EditorBlueprintResources/StandardMacros.IncrementInt` (`self.PaintedCount`))))))

(event `Has Won`
  (bind _returnvalue (`GameplayStatics.GetPlayerController` 0))
  (if (and (== (`self.UnpaintedCount`) 0) (== (`self.PurifiersCount`) 0))
    (bind _returnvalue_2 (`|CreateWidget` "/Game/AlphaNovaTest/UI/WBP_Win.WBP_Win_C"))
    (`UserWidget.AddToViewport` _returnvalue_2 0)
    (bind _foundwidgets (`WidgetBlueprintLibrary.GetAllWidgetsOfClass` "/Game/AlphaNovaTest/UI/WBP_TargetsInfo.WBP_TargetsInfo_C"))
    (`Widget.RemoveFromParent` _foundwidgets)
    (`self.DisableInput` (`Controller.K2_GetPawn` _returnvalue) (cast `/Game/AlphaNovaTest/Core/BP_PlayerController` _returnvalue :!pure true))))

(fn `UserConstructionScript`)